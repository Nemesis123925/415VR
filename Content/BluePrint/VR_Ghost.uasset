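; VR_Ghost is a ghost that wanders endlessly around the spot where it begins play.
; BeginPlay stores the start location, then a custom Roam event uses AI MoveTo toward a small random X/Y offset from that point.
; Each successful move calls Roam again, anchoring the wander to the origin; a failed move has no retry.
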(event Custom|Roam
  (bind _startlocation (Variables|Default|GetStartLocation))
  (AI|AIMoveTo 0 (Math|Vector|MakeVector (+ (.x _startlocation) (Math|Random|RandomFloatinRange -1e+01 1e+01)) (+ (.y _startlocation) (Math|Random|RandomFloatinRange -1e+01 1e+01)) 0.0) 0 5.0 false
    (:then
      (CallFunction|Roam))))

(event EventBeginPlay
  (Variables|Default|SetStartLocation (Transformation|GetActorLocation))
  (CallFunction|Roam))

(fn ConstructionScript)